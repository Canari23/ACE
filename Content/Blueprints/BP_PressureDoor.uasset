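; Pressure-plate double door that slides open once both its left and right trigger colliders are overlapped at the same time.
; Begin and end overlap events on each collider set a pair of flags, which Tick polls without filtering the overlapping actor.
; When both are set, it clears the left flag and disables both colliders, then a timeline lerps the panels apart, with no closing logic.
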(event OnComponentBeginOverlap(LeftCollider)
  (params (OverlappedComponent :type Primitive%20Component%20Object%20Reference) (OtherActor :type Actor%20Object%20Reference) (OtherComp :type Primitive%20Component%20Object%20Reference) (OtherBodyIndex :type Integer) (bFromSweep :type Boolean) (SweepResult :type Hit%20Result%20Structure%20%28by%20ref%29))
  (Variables|Default|SetLeftDown? true))

(event OnComponentEndOverlap(LeftCollider)
  (params (OverlappedComponent :type Primitive%20Component%20Object%20Reference) (OtherActor :type Actor%20Object%20Reference) (OtherComp :type Primitive%20Component%20Object%20Reference) (OtherBodyIndex :type Integer))
  (Variables|Default|SetLeftDown? false))

(event OnComponentBeginOverlap(RightCollider)
  (params (OverlappedComponent :type Primitive%20Component%20Object%20Reference) (OtherActor :type Actor%20Object%20Reference) (OtherComp :type Primitive%20Component%20Object%20Reference) (OtherBodyIndex :type Integer) (bFromSweep :type Boolean) (SweepResult :type Hit%20Result%20Structure%20%28by%20ref%29))
  (Variables|Default|SetRightDown? true))

(event OnComponentEndOverlap(RightCollider)
  (params (OverlappedComponent :type Primitive%20Component%20Object%20Reference) (OtherActor :type Actor%20Object%20Reference) (OtherComp :type Primitive%20Component%20Object%20Reference) (OtherBodyIndex :type Integer))
  (Variables|Default|SetRightDown? false))

(event EventBeginPlay)

(event Collision|EventActorBeginOverlap
  (params (OtherActor :type Actor%20Object%20Reference)))

(event EventTick
  (params (DeltaSeconds :type Float%20%28single-precision%29))
  (if (Variables|Default|GetLeftDown?)
    (if (Variables|Default|GetRightDown?)
      (Variables|Default|SetLeftDown? false)
      (Collision|SetCollisionEnabled (Variables|Default|GetRightCollider) "NoCollision")
      (Collision|SetCollisionEnabled (Variables|Default|GetLeftCollider) "NoCollision")
      (bind _newtrack_1 (Timeline|Timeline_0 PlayFromStart)
        (:Update
          (Transformation|SetRelativeLocation (Variables|Default|GetDoorLeft) (Math|Vector|Lerp(Vector) "-25.000000, 0,35.000000" "-80.000000, 0,35.000000" _newtrack_1) false false)
          (Transformation|SetRelativeLocation (Variables|Default|GetDoorRight) (Math|Vector|Lerp(Vector) "25.000000, 0,35.000000" "80.000000, 0,35.000000" _newtrack_1) false false))))))

(fn ConstructionScript)