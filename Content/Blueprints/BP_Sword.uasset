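; BP_Sword is a spinning sword pickup that triggers the win screen when touched.
; Tick continuously yaws the static mesh at a frame-rate-independent speed.
; Any actor overlapping the Box, unless its class is exactly BP_SimpleAI, creates the Win widget, adds it to the viewport, switches input to UI-only and shows the mouse cursor.
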(event OnComponentBeginOverlap(Box)
  (params (OverlappedComponent :type Primitive%20Component%20Object%20Reference) (OtherActor :type Actor%20Object%20Reference) (OtherComp :type Primitive%20Component%20Object%20Reference) (OtherBodyIndex :type Integer) (bFromSweep :type Boolean) (SweepResult :type Hit%20Result%20Structure%20%28by%20ref%29))
  (bind _returnvalue (Game|GetPlayerController 0))
  (if (not (== (Utilities|GetClass OtherActor) "/Game/Blueprints/AI/BP_SimpleAI.BP_SimpleAI_C"))
    (bind _returnvalue_2 (UserInterface|CreateWidget "/Game/Blueprints/UI/Win.Win_C"))
    (UserInterface|Viewport|AddtoViewport _returnvalue_2 0)
    (Input|SetInputModeUIOnly _returnvalue 0 "DoNotLock")
    (Variables|/Script/Engine.PlayerController|SetbShowMouseCursor _returnvalue true)))

(event EventBeginPlay)

(event Collision|EventActorBeginOverlap
  (params (OtherActor :type Actor%20Object%20Reference)))

(event EventTick
  (params (DeltaSeconds :type Float%20%28single-precision%29))
  (Transformation|AddLocalRotation (Variables|Default|GetStaticMesh) (Math|Rotator|MakeRotator 0.0 0.0 (* DeltaSeconds 2e+02)) false false))

(fn ConstructionScript)