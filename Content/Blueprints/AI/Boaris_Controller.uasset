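; AI controller for Boaris that runs the Boaris_BT behavior tree to drive patrolling and player detection.
; On BeginPlay it casts the pawn to BP_SimpleAI and seeds the blackboard with the patrol path's looping flag and an initial direction.
; AI Perception updates set CanSeePlayer whenever a BP_Pounce actor is sensed or lost.
; A node copying the path's wait time to the blackboard is disconnected and never runs.
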(event OnTargetPerceptionUpdated(AIPerception)
  (params (Actor :type Actor%20Object%20Reference) (Stimulus :type AI%20Stimulus%20Structure))
  (Utilities|Casting|CastToBP_Pounce Actor)
  (AI|Components|Blackboard|SetValueasBool (AI|GetBlackboard 0) (Utilities|Name|MakeLiteralName "CanSeePlayer") (.bSuccessfullySensed (Utilities|Struct|BreakAIStimulus Stimulus))))

(event EventBeginPlay
  (AI|RunBehaviorTree "/Game/Blueprints/AI/Boaris_BT.Boaris_BT")
  (bind _asbp_simple_ai (Utilities|Casting|CastToBP_SimpleAI (Pawn|GetControlledPawn)))
  (bind _output_get (Variables|Default|SetMyPawn _asbp_simple_ai))
  (AI|Components|Blackboard|SetValueasBool (AI|GetBlackboard 0) (Utilities|Name|MakeLiteralName "PathLooping") (Variables|/Game/Blueprints/AI/PatrolPaths/PatrolPath.PatrolPath_C|GetisLooping (Variables|/Game/Blueprints/AI/BP_SimpleAI.BP_SimpleAI_C|GetPatrolPath _output_get)))
  (Class|BlackboardComponent|SetValueasInt (AI|GetBlackboard 0) (Utilities|Name|MakeLiteralName "Direction") 1))

(fn ConstructionScript)