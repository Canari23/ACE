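; AI controller for Boaris that runs Boaris_BT on a BP_SimpleAI pawn and seeds its patrol looping and direction blackboard keys.
; Perception updates split stimuli by index: the first flags seeing BP_Pounce, a fresh second starts investigation, though target and sound locations are zero vectors.
; BeingCalled writes a called flag and location for the tree.
; CompleteSenses repeats the sense handling using real stimulus locations but is not called here.
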(event OnPerceptionUpdated(AIPerception)
  (params (UpdatedActors :type Array%20of%20Actor%20Object%20References))
  (for _array_element UpdatedActors
    (bind _info (Class|AIPerceptionComponent|GetActorsPerception (Variables|Default|GetAIPerception) _array_element))
    (for (_array_element_2 _array_index) (.lastsensedstimuli _info)
      (Variables|Default|SetSense _array_element_2)
      (switch int _array_index
        (:0
          (Utilities|Casting|CastToBP_Pounce (.target _info))
          (AI|Components|Blackboard|SetValueasBool (AI|GetBlackboard 0) (Utilities|Name|MakeLiteralName "CanSeePlayer") (.bsuccessfullysensed (Variables|Default|GetSense))))
        (:1
          (if (<= (.age (Variables|Default|GetSense)) 0.1)
            (AI|Components|Blackboard|SetValueasBool (AI|GetBlackboard 0) (Utilities|Name|MakeLiteralName "isInvestigating") (.bsuccessfullysensed (Variables|Default|GetSense)))
            (AI|Components|Blackboard|SetValueasVector (AI|GetBlackboard 0) (Utilities|Name|MakeLiteralName "TargetLocation") "0, 0, 0")
            ;[1 1 1] Boaris can say something
            (Audio|PlaySoundatLocation 0 "0, 0, 0" "0, 0, 0" 1.0 1.0 0.0 0 0 0)))))))

(event Custom|BeingCalled
  (params (BoolValue :type Boolean) (VectorValue :type Vector))
  (bind _returnvalue (AI|GetBlackboard 0))
  ;[1 1 1] Value for Called node on the BT
  (AI|Components|Blackboard|SetValueasBool _returnvalue (Utilities|Name|MakeLiteralName "Called") BoolValue)
  (AI|Components|Blackboard|SetValueasVector _returnvalue (Utilities|Name|MakeLiteralName "TargetLocation") VectorValue))

(event EventBeginPlay
  (AI|RunBehaviorTree "/Game/Blueprints/Boaris_AI/Boaris_BT.Boaris_BT")
  (bind _asbp_simple_ai (Utilities|Casting|CastToBP_SimpleAI (Pawn|GetControlledPawn)))
  (bind _output_get (Variables|Default|SetMyPawn _asbp_simple_ai))
  (AI|Components|Blackboard|SetValueasBool (AI|GetBlackboard 0) (Utilities|Name|MakeLiteralName "PathLooping") (Variables|/Game/Blueprints/Boaris_AI/PatrolPaths/PatrolPath.PatrolPath_C|GetisLooping (Variables|/Game/Blueprints/Boaris_AI/BP_SimpleAI.BP_SimpleAI_C|GetPatrolPath _output_get)))
  (Class|BlackboardComponent|SetValueasInt (AI|GetBlackboard 0) (Utilities|Name|MakeLiteralName "Direction") 1))

(fn ConstructionScript)

(fn CompleteSenses
  (params (Array :type Array%20of%20AI%20Stimulus%20Structures))
  (for (_array_element _array_index) Array
    (LocalVariables|SetLocal%20Sense _array_element)
    (switch int _array_index
      (:0
        (AI|Components|Blackboard|SetValueasBool (AI|GetBlackboard 0) (Utilities|Name|MakeLiteralName "CanSeePlayer") (.bsuccessfullysensed (LocalVariables|GetLocal%20Sense))))
      (:1
        (AI|Components|Blackboard|SetValueasBool (AI|GetBlackboard 0) (Utilities|Name|MakeLiteralName "isInvestigating") (.bsuccessfullysensed (LocalVariables|GetLocal%20Sense)))
        (AI|Components|Blackboard|SetValueasVector (AI|GetBlackboard 0) (Utilities|Name|MakeLiteralName "TargetLocation") (.stimuluslocation (LocalVariables|GetLocal%20Sense)))
        ;[1 1 1] Boaris can say something
        (Audio|PlaySoundatLocation 0 (.stimuluslocation (LocalVariables|GetLocal%20Sense)) "0, 0, 0" 1.0 1.0 0.0 0 0 0)))))