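; BP_SimpleAI is a simple enemy that can be damaged and killed by BP_Pounce's attack, with no movement or decision logic.
; Any actor overlap spawns an emitter and plays a stomach-hit animation.
; A capsule overlap with an attacking BP_Pounce prints a tail-hit message and reduces Health.
; At zero Health it starts the knockout animation and is destroyed immediately, as the Delay node is unconnected.
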(event OnComponentBeginOverlap(CapsuleComponent)
  (params (OverlappedComponent :type Primitive%20Component%20Object%20Reference) (OtherActor :type Actor%20Object%20Reference) (OtherComp :type Primitive%20Component%20Object%20Reference) (OtherBodyIndex :type Integer) (bFromSweep :type Boolean) (SweepResult :type Hit%20Result%20Structure%20%28by%20ref%29))
  (bind _asbp_pounce (Utilities|Casting|CastToBP_Pounce OtherActor))
  (if (Variables|/Game/Blueprints/BP_Pounce.BP_Pounce_C|GetAttack _asbp_pounce)
    (Development|PrintString "Hit with Tail")
    (bind _output_get (Variables|Default|SetHealth (- (Variables|Default|GetHealth) 0.25)))
    (if (<= _output_get 0.0)
      (CallFunction|Death)
      (Actor|DestroyActor))))

(event EventBeginPlay)

(event Collision|EventActorBeginOverlap
  (params (OtherActor :type Actor%20Object%20Reference))
  (CallFunction|TakeDamage))

(event EventTick
  (params (DeltaSeconds :type Float%20%28single-precision%29)))

(fn ConstructionScript)

(fn TakeDamage
  (Effects|SpawnEmitteratLocation 0 (Transformation|GetActorLocation))
  (Components|Animation|PlayAnimation (Variables|Character|GetMesh) "/Game/Characters/Boaris/Animations/MixamoAnims/Stomach_Hit.Stomach_Hit" false))

(fn Death
  (Components|Animation|PlayAnimation (Variables|Character|GetMesh) "/Game/Characters/Boaris/Animations/MixamoAnims/Knocked_Out.Knocked_Out" false))