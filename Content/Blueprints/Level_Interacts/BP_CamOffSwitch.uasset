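; BP_CamOffSwitch is a level interactable that shuts off all Camera_BP actors when triggered with BP_Nyx nearby.
; A Box overlap sets IsNear when the actor is exactly BP_Nyx, and any end overlap clears it.
; The TurnOff event checks IsNear, then gathers every Camera_BP through GetAllActorsOfClass and calls TurnOff on them.
; Nothing in this Blueprint calls its own TurnOff event.
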(event OnComponentBeginOverlap(Box)
  (params (OverlappedComponent :type Primitive%20Component%20Object%20Reference) (OtherActor :type Actor%20Object%20Reference) (OtherComp :type Primitive%20Component%20Object%20Reference) (OtherBodyIndex :type Integer) (bFromSweep :type Boolean) (SweepResult :type Hit%20Result%20Structure%20%28by%20ref%29))
  (if (== (Utilities|GetClass OtherActor) "/Game/Blueprints/BP_Nyx.BP_Nyx_C")
    (Variables|Default|SetIsNear? true)))

(event OnComponentEndOverlap(Box)
  (params (OverlappedComponent :type Primitive%20Component%20Object%20Reference) (OtherActor :type Actor%20Object%20Reference) (OtherComp :type Primitive%20Component%20Object%20Reference) (OtherBodyIndex :type Integer))
  (Variables|Default|SetIsNear? false))

(event Custom|TurnOff
  (if (Variables|Default|GetIsNear?)
    (bind _outactors (Actor|GetAllActorsOfClass "/Game/Blueprints/SecurityCam_AI/Camera_BP.Camera_BP_C"))
    (Default|TurnOff _outactors)))

(event EventBeginPlay)

(event Collision|EventActorBeginOverlap
  (params (OtherActor :type Actor%20Object%20Reference)))

(event EventTick
  (params (DeltaSeconds :type Float%20%28single-precision%29)))

(fn ConstructionScript)